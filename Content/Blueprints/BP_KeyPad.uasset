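; BP_KeyPad is a keypad actor that opens a code lock UI when the third-person character enters its box trigger while that character's IsPowerOn flag is set.
; Opening the lock switches to UI-only input with a visible cursor and disables player movement; without power, a need-power widget appears instead.
; A DoOnce prevents duplicate code lock widgets and resets after a short delay when the character leaves the box.
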(event `self.Box.OnComponentBeginOverlap`
  (params (OverlappedComponent :type "PrimitiveComponent Object Reference") (OtherActor :type "Actor Object Reference") (OtherComp :type "PrimitiveComponent Object Reference") (OtherBodyIndex :type Integer) (bFromSweep :type Boolean) (SweepResult :type "HitResult Structure (by ref)"))
  (bind _returnvalue (`GameplayStatics.GetPlayerController` 0))
  (bind _asthird_person_character (cast `/Game/ThirdPersonBP/Blueprints/ThirdPersonCharacter` OtherActor))
  (if (`/Game/ThirdPersonBP/Blueprints/ThirdPersonCharacter.IsPowerOn?` _asthird_person_character)
    (`/Engine/EditorBlueprintResources/StandardMacros.DoOnce` false :!label _label
      (:`Completed`
        (bind _returnvalue_2 (`|CreateWidget` "/Game/UMG/Widget_CodeLock.Widget_CodeLock_C"))
        (`UserWidget.AddToViewport` _returnvalue_2 0)
        (`WidgetBlueprintLibrary.SetInputMode_UIOnlyEx` _returnvalue _returnvalue_2)
        (bind _asthird_person_character_2 (cast `/Game/ThirdPersonBP/Blueprints/ThirdPersonCharacter` (`GameplayStatics.GetPlayerCharacter` 0)))
        (`CharacterMovementComponent.DisableMovement` (`Character.CharacterMovement` _asthird_person_character_2))
        (set `PlayerController.bShowMouseCursor` true _returnvalue)))
    (else
      (bind _returnvalue_3 (`|CreateWidget` "/Game/UMG/Widget_NeedPowerOn.Widget_NeedPowerOn_C"))
      (`UserWidget.AddToViewport` _returnvalue_3 0))))

(event `self.Box.OnComponentEndOverlap`
  (params (OverlappedComponent :type "PrimitiveComponent Object Reference") (OtherActor :type "Actor Object Reference") (OtherComp :type "PrimitiveComponent Object Reference") (OtherBodyIndex :type Integer))
  (cast `/Game/ThirdPersonBP/Blueprints/ThirdPersonCharacter` OtherActor)
  (`KismetSystemLibrary.Delay` 1.0)
  (goto _label :!via `Reset`))

(fn `UserConstructionScript`)