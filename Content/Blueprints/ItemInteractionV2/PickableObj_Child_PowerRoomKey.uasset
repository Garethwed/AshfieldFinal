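; Pickable key item for the power room, a child of the pickable object Blueprint that the player collects into their inventory.
; On PickUp it adds one of its item to the interacter's InventoryComponent.
; If that succeeds, it destroys itself, prints a debug message and calls HasPowerKey on the interacting ThirdPersonCharacter.
; UseItem and the construction script only defer to the parent.
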(event `self.PickUp`
  (params (Interacter :type "Actor Object Reference"))
  (bind _success (`/Game/InventorySystem/InventoryComponent.AddToInventory` (`self.GetComponentByClass` Interacter "/Game/InventorySystem/InventoryComponent.InventoryComponent_C") (make `/Game/InventorySystem/SlotStructure` (`self.ItemStructure`) 1)))
  (if _success
    (`self.K2_DestroyActor`)
    (bind _asthird_person_character (cast `/Game/ThirdPersonBP/Blueprints/ThirdPersonCharacter` Interacter))
    (`KismetSystemLibrary.PrintString` "key pickup")
    (`/Game/ThirdPersonBP/Blueprints/ThirdPersonCharacter.HasPowerKey` _asthird_person_character)))

(fn `Use Item`
  (returns (Succcess :type Boolean))
  (bind _succcess (`parent.Use Item`))
  (return _succcess))

(fn `UserConstructionScript`
  (`parent.UserConstructionScript`))