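; Inspectable creepy doll from the item interaction system that turns its head when inspected.
; The Inspection event stores the actor's rotation, then uses a DoOnce to play the HeadRotation timeline a single time.
; Each timeline update combines the animated yaw with that stored world rotation and sets it as the Head component's relative rotation.
; The Inspect Function is a stub that returns false.
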(event `Inspection`
  ;[1 1 1] Init
  (set `self.HeadIni` (`self.K2_GetActorRotation`))
  (`/Engine/EditorBlueprintResources/StandardMacros.DoOnce` false
    (:`Completed`
      (bind (_direction _newtrack_0) (`Timeline|Head rotation`)
        (:`Update`
          (`SceneComponent.K2_SetRelativeRotation` (`self.head`) (`KismetMathLibrary.ComposeRotators` (`KismetMathLibrary.MakeRotator` 0.0 0.0 _newtrack_0) (`self.HeadIni`)) false false))))))

(fn `Inspect Function`
  (returns (Success :type Boolean) (Success :type Boolean))
  (return false false))

(fn `UserConstructionScript`
  (`parent.UserConstructionScript`))