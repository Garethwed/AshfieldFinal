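; Door actor that a player inside its trigger box can open and close with Interact when their inventory holds the matching key.
; The trigger enables input and shows a prompt widget, and Interact searches the character's InventoryComponent for KeyName.
; A match flip-flops a timeline that rotates the door from its initial rotation, with door and lock sounds.
; Distance checks during rotation and on Tick disable input and hide or remove the prompt.
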(event `self.Trigger.OnComponentBeginOverlap`
  (params (OverlappedComponent :type "PrimitiveComponent Object Reference") (OtherActor :type "Actor Object Reference") (OtherComp :type "PrimitiveComponent Object Reference") (OtherBodyIndex :type Integer) (bFromSweep :type Boolean) (SweepResult :type "HitResult Structure (by ref)"))
  ;[1 1 1] Triggerbox
  (`self.EnableInput` (`GameplayStatics.GetPlayerController` 0))
  (`/Engine/EditorBlueprintResources/StandardMacros.DoOnce` false :!label _label
    (:`Completed`
      (bind _returnvalue (`|CreateWidget` "/Game/Blueprints/Doors/MessageNearTheDoorWithKey.MessageNearTheDoorWithKey_C" (`GameplayStatics.GetPlayerController` 0) self))
      (bind _output_get (set `self.HelpingWidget` _returnvalue))
      (`UserWidget.AddToViewport` _output_get 0))))

(event `self.Trigger.OnComponentEndOverlap`
  (params (OverlappedComponent :type "PrimitiveComponent Object Reference") (OtherActor :type "Actor Object Reference") (OtherComp :type "PrimitiveComponent Object Reference") (OtherBodyIndex :type Integer))
  ;[1 1 1] Triggerbox
  (`self.DisableInput` (`GameplayStatics.GetPlayerController` 0))
  (`Widget.RemoveFromParent` (`self.HelpingWidget`))
  (goto _label :!via `Reset`))

(event `InputAction|Interact`
  (params (Key :type "Key Structure"))
  (bind _returnvalue (`GameplayStatics.GetPlayerController` 0))
  (bind _helpingwidget (`self.HelpingWidget`))
  ;[1 1 1] key condition
  (:`Pressed`
    (bind _asthird_person_character (cast `/Game/ThirdPersonBP/Blueprints/ThirdPersonCharacter` (`GameplayStatics.GetPlayerCharacter` 0)))
    (for _array_element (`/Game/InventorySystem/InventoryComponent.Inventory` (`/Game/ThirdPersonBP/Blueprints/ThirdPersonCharacter.InventoryComponent` _asthird_person_character))
      (bind _returnvalue_2 (`KismetTextLibrary.EqualEqual_TextText` (break `/Game/InventorySystem/ItemStructure` (break `/Game/InventorySystem/SlotStructure` _array_element)) (`self.KeyName`)))
      (if _returnvalue_2
        (break)))
    (`|ExecutionSequence`
      (:`then_0`
        (if _returnvalue_2
          ;[1 1 1] Configure rotator
          (`/Engine/EditorBlueprintResources/StandardMacros.FlipFlop`
            (:`A`
              (bind (_direction _door_rotation) (`Timeline|Rotation` :!label _label_2)
                (:`Update`
                  (`self.K2_SetActorRelativeRotation` (`KismetMathLibrary.ComposeRotators` (`KismetMathLibrary.MakeRotator` 0.0 0.0 _door_rotation) (`self.Porte_ini`)))
                  ;;[1 1 1] BugFixWhileItRotates
                  (if (>= (`self.GetDistanceTo` (`GameplayStatics.GetPlayerCharacter` 0)) 300.0)
                    (`self.DisableInput` _returnvalue)
                    (`Widget.SetVisibility` _helpingwidget "Hidden")
                    (else
                      (`self.EnableInput` _returnvalue)
                      (`Widget.SetVisibility` _helpingwidget "Visible"))))
                (:`Finished`
                  (`GameplayStatics.PlaySoundAtLocation` "/Game/ZActorSounds/door-5-open.door-5-open" (0.0 0.0 0.0) (struct) 1.0 1.0 0.0 null null null))))
            (:`B`
              (goto _label_2 :!via `Reverse`)))))
      (:`then_1`
        (`/Engine/EditorBlueprintResources/StandardMacros.DoOnce` false
          (:`Completed`
            (`GameplayStatics.PlaySoundAtLocation` "/Game/ZActorSounds/door-lock-1.door-lock-1" (0.0 0.0 0.0) (struct) 1.0 1.0 0.0 null null null)))))))

(event `self.ReceiveBeginPlay`
  ;[1 1 1] Init
  (set `self.Porte_ini` (`self.K2_GetActorRotation`)))

(event `self.ReceiveTick`
  (params (DeltaSeconds :type "Float (single-precision)"))
  ;[1 1 1] BugFix
  (if (>= (`self.GetDistanceTo` (`GameplayStatics.GetPlayerCharacter` 0)) 500.0)
    (`self.HelpingWidget`
      (:`then`
        (`self.DisableInput` (`GameplayStatics.GetPlayerController` 0))
        (`Widget.RemoveFromParent` (`self.HelpingWidget`)))
      (:`else`))))

(fn `UserConstructionScript`)