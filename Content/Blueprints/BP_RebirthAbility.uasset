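; Rebirth ability actor that temporarily banishes zombies or the RunatPlayer character entering its hitbox by teleporting them high overhead.
; Hitbox overlap runs a cast chain over five character classes, lifting the match by a fixed height, then teleporting it again after a delay.
; ZombieTut drops relative to its own position, while the others land relative to this actor's location, lowered by the same offset.
; An older BasicAICharacter branch remains unconnected.
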(event `self.Hitbox.OnComponentBeginOverlap`
  (params (OverlappedComponent :type "PrimitiveComponent Object Reference") (OtherActor :type "Actor Object Reference") (OtherComp :type "PrimitiveComponent Object Reference") (OtherBodyIndex :type Integer) (bFromSweep :type Boolean) (SweepResult :type "HitResult Structure (by ref)"))
  (bind (_returnvalue_x _returnvalue_y _returnvalue_z) (`KismetMathLibrary.BreakVector` (`self.K2_GetActorLocation`)))
  (bind (_returnvalue_x_2 _returnvalue_y_2 _returnvalue_z_2) (`KismetMathLibrary.BreakVector` (`self.K2_GetActorLocation`)))
  (bind (_returnvalue_x_3 _returnvalue_y_3 _returnvalue_z_3) (`KismetMathLibrary.BreakVector` (`self.K2_GetActorLocation`)))
  (bind (_returnvalue_x_4 _returnvalue_y_4 _returnvalue_z_4) (`KismetMathLibrary.BreakVector` (`self.K2_GetActorLocation`)))
  (bind _aszombie_tut (cast `/Game/Blueprints/ChaseRoamEnemy/ZombieTut` OtherActor)
    (:`then`
      (bind (_returnvalue_x_5 _returnvalue_y_5 _returnvalue_z_5) (`KismetMathLibrary.BreakVector` (`self.K2_GetActorLocation` _aszombie_tut)))
      (`self.K2_TeleportTo` :`self` _aszombie_tut :`DestLocation` (`KismetMathLibrary.MakeVector` _returnvalue_x_5 _returnvalue_y_5 (+ 2090.0 _returnvalue_z_5)))
      (`KismetSystemLibrary.Delay` 15.0)
      (bind (_returnvalue_x_6 _returnvalue_y_6 _returnvalue_z_6) (`KismetMathLibrary.BreakVector` (`self.K2_GetActorLocation` _aszombie_tut)))
      (`self.K2_TeleportTo` :`self` _aszombie_tut :`DestLocation` (`KismetMathLibrary.MakeVector` _returnvalue_x_6 _returnvalue_y_6 (- _returnvalue_z_6 2090.0))))
    (:`CastFailed`
      (bind _asrunat_player (cast `/Game/Blueprints/EnemyWithTarget/RunatPlayer` OtherActor)
        (:`then`
          (bind (_returnvalue_x_7 _returnvalue_y_7 _returnvalue_z_7) (`KismetMathLibrary.BreakVector` (`self.K2_GetActorLocation` _asrunat_player)))
          (`self.K2_TeleportTo` :`self` _asrunat_player :`DestLocation` (`KismetMathLibrary.MakeVector` _returnvalue_x_7 _returnvalue_y_7 (+ 2090.0 _returnvalue_z_7)))
          (`KismetSystemLibrary.Delay` 15.0)
          (`self.K2_TeleportTo` :`self` _asrunat_player :`DestLocation` (`KismetMathLibrary.MakeVector` _returnvalue_x_2 _returnvalue_y_2 (- _returnvalue_z_2 2090.0))))
        (:`CastFailed`
          (bind _aszombie_1bp (cast `/Game/NPC/Enemy_1/Zombie1BP` OtherActor)
            (:`then`
              (bind (_returnvalue_x_8 _returnvalue_y_8 _returnvalue_z_8) (`KismetMathLibrary.BreakVector` (`self.K2_GetActorLocation` _aszombie_1bp)))
              (`self.K2_TeleportTo` :`self` _aszombie_1bp :`DestLocation` (`KismetMathLibrary.MakeVector` _returnvalue_x_8 _returnvalue_y_8 (+ 2090.0 _returnvalue_z_8)))
              (`KismetSystemLibrary.Delay` 15.0)
              (`self.K2_TeleportTo` :`self` _aszombie_1bp :`DestLocation` (`KismetMathLibrary.MakeVector` _returnvalue_x_3 _returnvalue_y_3 (- _returnvalue_z_3 2090.0))))
            (:`CastFailed`
              (bind _aszombie_2bp (cast `/Game/NPC/Enemy_2/Zombie2bp` OtherActor)
                (:`then`
                  (bind (_returnvalue_x_9 _returnvalue_y_9 _returnvalue_z_9) (`KismetMathLibrary.BreakVector` (`self.K2_GetActorLocation` _aszombie_2bp)))
                  (`self.K2_TeleportTo` :`self` _aszombie_2bp :`DestLocation` (`KismetMathLibrary.MakeVector` _returnvalue_x_9 _returnvalue_y_9 (+ 2090.0 _returnvalue_z_9)))
                  (`KismetSystemLibrary.Delay` 15.0)
                  (`self.K2_TeleportTo` :`self` _aszombie_2bp :`DestLocation` (`KismetMathLibrary.MakeVector` _returnvalue_x_4 _returnvalue_y_4 (- _returnvalue_z_4 2090.0))))
                (:`CastFailed`
                  (bind _aszombie_3bp (cast `/Game/NPC/Enemy_3/Zombie3BP` OtherActor))
                  (bind (_returnvalue_x_10 _returnvalue_y_10 _returnvalue_z_10) (`KismetMathLibrary.BreakVector` (`self.K2_GetActorLocation` _aszombie_3bp)))
                  (`self.K2_TeleportTo` :`self` _aszombie_3bp :`DestLocation` (`KismetMathLibrary.MakeVector` _returnvalue_x_10 _returnvalue_y_10 (+ 2090.0 _returnvalue_z_10)))
                  (`KismetSystemLibrary.Delay` 15.0)
                  (`self.K2_TeleportTo` :`self` _aszombie_3bp :`DestLocation` (`KismetMathLibrary.MakeVector` _returnvalue_x _returnvalue_y (- _returnvalue_z 2090.0))))))))))))

(fn `UserConstructionScript`)