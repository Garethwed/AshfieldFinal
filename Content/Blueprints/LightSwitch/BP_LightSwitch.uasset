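; BP_LightSwitch is a switch that lets a player with the key turn on the power.
; Overlapping PlayerRange while HasKey is set flags the player in range and shows a prompt widget once, until overlap end clears both.
; ToggleLights, when in range, brightens each entry in Lights, adds a power-on widget per light and sets IsPowerOn on ThirdPersonCharacter.
; The switch-off branch does nothing because its dimming nodes are disconnected.
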(event `self.PlayerRange.OnComponentBeginOverlap`
  (params (OverlappedComponent :type "PrimitiveComponent Object Reference") (OtherActor :type "Actor Object Reference") (OtherComp :type "PrimitiveComponent Object Reference") (OtherBodyIndex :type Integer) (bFromSweep :type Boolean) (SweepResult :type "HitResult Structure (by ref)"))
  (if (`self.HasKey`)
    (`/Engine/EditorBlueprintResources/StandardMacros.DoOnce` false :!label _label
      (:`Completed`
        (set `self.IsinRange` true)
        (bind _returnvalue (`|CreateWidget` "/Game/Blueprints/LightSwitch/MessageNearLight.MessageNearLight_C"))
        (`UserWidget.AddToViewport` _returnvalue 0)))))

(event `self.PlayerRange.OnComponentEndOverlap`
  (params (OverlappedComponent :type "PrimitiveComponent Object Reference") (OtherActor :type "Actor Object Reference") (OtherComp :type "PrimitiveComponent Object Reference") (OtherBodyIndex :type Integer))
  (if (`self.HasKey`)
    (`Widget.RemoveFromParent` (stale `self.PlayerRange.OnComponentBeginOverlap` _returnvalue))
    (set `self.IsinRange` false)
    (goto _label :!via `Reset`)))

(fn `ToggleLights`
  (if (`self.IsinRange`)
    (if (`self.IsLightOn`)
      (for _ (`self.Lights`)
        _)
      (else
        (for _array_element (`self.Lights`)
          (`LightComponent.SetIntensity` (`Light.LightComponent` _array_element) 30.0)
          (set `self.IsLightOn` true)
          (bind _returnvalue (`|CreateWidget` "/Game/UMG/widgetPoweron.widgetPoweron_C"))
          (`UserWidget.AddToViewport` _returnvalue 0)
          (bind _asthird_person_character (cast `/Game/ThirdPersonBP/Blueprints/ThirdPersonCharacter` (`GameplayStatics.GetPlayerCharacter` 0)))
          (set `/Game/ThirdPersonBP/Blueprints/ThirdPersonCharacter.IsPowerOn?` true _asthird_person_character))))))

(fn `UserConstructionScript`)