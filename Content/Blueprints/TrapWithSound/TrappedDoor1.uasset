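; Interactive door Blueprint that springs a trap on the player, after which it requires a key to open.
; A trigger box enables input and shows a help widget, and Interact toggles the door through a rotation timeline.
; Tick watches a second trigger that, once, sets Trapped, plays a laugh and reverses an open door, later slammed audibly.
; When trapped, Interact searches the character's inventory for KeyName; distance checks patch input and widget state.
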(event `self.Trigger.OnComponentBeginOverlap`
  (params (OverlappedComponent :type "PrimitiveComponent Object Reference") (OtherActor :type "Actor Object Reference") (OtherComp :type "PrimitiveComponent Object Reference") (OtherBodyIndex :type Integer) (bFromSweep :type Boolean) (SweepResult :type "HitResult Structure (by ref)"))
  ;[1 1 1] Triggerbox
  (`self.EnableInput` (`GameplayStatics.GetPlayerController` 0))
  (`/Engine/EditorBlueprintResources/StandardMacros.DoOnce` false :!label _label
    (:`Completed`
      (bind _returnvalue (`|CreateWidget` "/Game/Blueprints/TrapWithSound/MessageNearTheTrappedDoor.MessageNearTheTrappedDoor_C" (`GameplayStatics.GetPlayerController` 0) self))
      (bind _output_get (set `self.HelpingWidget` _returnvalue))
      (`UserWidget.AddToViewport` _output_get 0))))

(event `self.Trigger.OnComponentEndOverlap`
  (params (OverlappedComponent :type "PrimitiveComponent Object Reference") (OtherActor :type "Actor Object Reference") (OtherComp :type "PrimitiveComponent Object Reference") (OtherBodyIndex :type Integer))
  ;[1 1 1] Triggerbox
  (`self.DisableInput` (`GameplayStatics.GetPlayerController` 0))
  (`Widget.RemoveFromParent` (`self.HelpingWidget`))
  (goto _label :!via `Reset`))

(event `InputAction|Interact`
  (params (Key :type "Key Structure"))
  (bind _returnvalue (`GameplayStatics.GetPlayerController` 0))
  (bind _helpingwidget (`self.HelpingWidget`))
  (:`Pressed`
    (if (`self.Trapped?`)
      ;[1 1 1] key condition
      (bind _asthird_person_character (cast `/Game/ThirdPersonBP/Blueprints/ThirdPersonCharacter` (`GameplayStatics.GetPlayerCharacter` 0)))
      (for _array_element (`/Game/InventorySystem/InventoryComponent.Inventory` (`/Game/ThirdPersonBP/Blueprints/ThirdPersonCharacter.InventoryComponent` _asthird_person_character))
        (bind _returnvalue_2 (`KismetTextLibrary.EqualEqual_TextText` (break `/Game/InventorySystem/ItemStructure` (break `/Game/InventorySystem/SlotStructure` _array_element)) (`self.KeyName`)))
        (if _returnvalue_2
          (break)))
      (if _returnvalue_2
        ;[1 1 1] Configure rotator
        (`/Engine/EditorBlueprintResources/StandardMacros.FlipFlop` :!label _label_2
          (:`A`
            (set `self.Opened?` true)
            (bind (_direction _door_rotation) (`Timeline|Rotation` :!label _label_3)
              (:`Update`
                (`SceneComponent.K2_SetRelativeRotation` (`self.Door`) (`KismetMathLibrary.ComposeRotators` (`KismetMathLibrary.MakeRotator` 0.0 0.0 _door_rotation) (`self.Porte_ini`)) false false)
                ;;[1 1 1] BugFixWhileItRotates
                (if (>= (`self.GetDistanceTo` (`GameplayStatics.GetPlayerCharacter` 0)) 400.0)
                  (`self.DisableInput` _returnvalue)
                  (`Widget.SetVisibility` _helpingwidget "Hidden")
                  (elif (not (`self.Trapped?`))
                    (`self.EnableInput` _returnvalue)
                    (`Widget.SetVisibility` _helpingwidget "Visible"))))
              (:`Finished`
                (if (not (>= (`self.GetDistanceTo` (`GameplayStatics.GetPlayerCharacter` 0)) 400.0))
                  (`self.EnableInput` (`GameplayStatics.GetPlayerCharacter` 0) null))
                (if (`self.Trapped?`)
                  (`/Engine/EditorBlueprintResources/StandardMacros.DoOnce` false
                    (:`Completed`
                      (`GameplayStatics.PlaySoundAtLocation` "/Game/Blueprints/TrapWithSound/Claquement_de_porte.Claquement_de_porte" (0.0 0.0 0.0) (struct) 1.0 1.0 0.0 null null null)))))))
          (:`B`
            (set `self.Opened?` false)
            (goto _label_3 :!via `Reverse`)))
        (else
          (`KismetSystemLibrary.PrintString` (`KismetTextLibrary.Conv_TextToString` (`self.KeyName`)))
          (`KismetSystemLibrary.PrintString` "You need the key for ")))
      (else
        (goto _label_2)))))

(event `self.ReceiveBeginPlay`
  ;[1 1 1] Init
  (set `self.Porte_ini` (`self.K2_GetActorRotation`)))

(event `self.ReceiveTick`
  (params (DeltaSeconds :type "Float (single-precision)"))
  ;[1 1 1] BugFix
  (`|ExecutionSequence`
    (:`then_0`
      (if (>= (`self.GetDistanceTo` (`GameplayStatics.GetPlayerCharacter` 0)) 400.0)
        (`self.HelpingWidget`
          (:`then`
            (`self.DisableInput` (`GameplayStatics.GetPlayerController` 0))
            (`Widget.RemoveFromParent` (`self.HelpingWidget`)))
          (:`else`))))
    (:`then_1`
      ;[1 1 1] TrapSetup
      (`/Engine/EditorBlueprintResources/StandardMacros.DoOnce` false :!label _label_4
        (:`Completed`
          (if (`PrimitiveComponent.IsOverlappingActor` (`self.TriggerTheTrap`) (`GameplayStatics.GetPlayerCharacter` 0))
            (set `self.Trapped?` true)
            (`GameplayStatics.PlaySoundAtLocation` "/Game/Blueprints/TrapWithSound/Laught.Laught" (0.0 0.0 0.0) (struct) 1.0 1.0 0.0 null null null)
            (if (`self.Opened?`)
              (`self.DisableInput` (`GameplayStatics.GetPlayerController` 0))
              (goto _label_3 :!via `Reverse`))
            (else
              (goto _label_4 :!via `Reset`))))))))

(fn `UserConstructionScript`)