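; Crucifix actor that rotates once when something overlaps its Box trigger.
; BeginPlay stores the starting rotation, and the first overlap by any actor plays the Rotation timeline through a DoOnce that is never reset.
; Each update combines the timeline's DoorRotation value, as roll, with that starting rotation and applies it to the whole actor.
; An alternative that rotates only the static mesh is left unconnected.
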(event `self.Box.OnComponentBeginOverlap`
  (params (OverlappedComponent :type "PrimitiveComponent Object Reference") (OtherActor :type "Actor Object Reference") (OtherComp :type "PrimitiveComponent Object Reference") (OtherBodyIndex :type Integer) (bFromSweep :type Boolean) (SweepResult :type "HitResult Structure (by ref)"))
  (`/Engine/EditorBlueprintResources/StandardMacros.DoOnce` false
    (:`Completed`
      ;[1 1 1] Rotation
      (bind (_direction _door_rotation) (`Timeline|Rotation`)
        (:`Update`
          (`self.K2_SetActorRotation` self (`KismetMathLibrary.ComposeRotators` (`KismetMathLibrary.MakeRotator` _door_rotation) (`self.InitRotator`)) false))))))

(event `self.ReceiveBeginPlay`
  ;[1 1 1] Init
  (set `self.InitRotator` (`self.K2_GetActorRotation`)))

(fn `UserConstructionScript`)