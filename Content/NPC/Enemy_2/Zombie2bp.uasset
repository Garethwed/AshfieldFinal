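; Enemy zombie character that chases the player on sight and kills them at melee range.
; Pawn sensing triggers an AI move toward the seen player; arrival starts a timed, re-entry-guarded attack.
; After the windup delay, it calls the player's death event only if the mesh overlap flag still marks them in contact.
; Walk and Run events switch the movement speed.
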(event `self.PawnSensing.OnSeePawn`
  (params (Pawn :type "Pawn Object Reference"))
  (bind _asthird_person_character (cast `/Game/ThirdPersonBP/Blueprints/ThirdPersonCharacter` Pawn))
  (`|AIMoveTo` self (0.0 0.0 0.0) _asthird_person_character 45.0
    (:`OnSuccess`
      (if (not (`self.Attacking`))
        (set `self.Attacking` true)
        (`KismetSystemLibrary.Delay` 1.3)
        (if (`self.Kill?`)
          (bind _asthird_person_character_2 (cast `/Game/ThirdPersonBP/Blueprints/ThirdPersonCharacter` (`GameplayStatics.GetPlayerCharacter` 0)))
          (`/Game/ThirdPersonBP/Blueprints/ThirdPersonCharacter.DeathEvent` _asthird_person_character_2))
        (`KismetSystemLibrary.Delay` 0.5)
        (set `self.Attacking` false)))))

(event `Walk`
  (set `CharacterMovementComponent.MaxWalkSpeed` 150.0 (`self.CharacterMovement`)))

(event `self.Mesh.OnComponentBeginOverlap`
  (params (OverlappedComponent :type "PrimitiveComponent Object Reference") (OtherActor :type "Actor Object Reference") (OtherComp :type "PrimitiveComponent Object Reference") (OtherBodyIndex :type Integer) (bFromSweep :type Boolean) (SweepResult :type "HitResult Structure (by ref)"))
  (cast `/Game/ThirdPersonBP/Blueprints/ThirdPersonCharacter` OtherActor)
  (set `self.Kill?` true))

(event `Run`
  (set `CharacterMovementComponent.MaxWalkSpeed` 450.0 (`self.CharacterMovement`)))

(event `self.Mesh.OnComponentEndOverlap`
  (params (OverlappedComponent :type "PrimitiveComponent Object Reference") (OtherActor :type "Actor Object Reference") (OtherComp :type "PrimitiveComponent Object Reference") (OtherBodyIndex :type Integer))
  (set `self.Kill?` false))

(fn `UserConstructionScript`)